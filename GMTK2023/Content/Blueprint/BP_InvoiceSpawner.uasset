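; BP_InvoiceSpawner is an actor that keeps spawning BP_Invoice actors into a growing stack at its InvoiceSpawnLocation.
; The first invoice spawns on BeginPlay, and each spawn sets a one-shot timer with a random delay between MinSpawnTime and MaxSpawnTime that triggers the next.
; Each invoice sits OffsetAmount higher than the last via an incrementing OffsetCount and gets a random yaw.
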(event Custom|SpawnInvoice
  (bind _invoicespawnlocation (Variables|Default|GetInvoiceSpawnLocation))
  (bind _returnvalue (Transformation|GetWorldTransform _invoicespawnlocation))
  (bind (_roll _pitch _yaw) (Math|Rotator|BreakRotator (.rotation _returnvalue)))
  (Game|SpawnActorfromClass "/Game/Blueprint/BP_Invoice.BP_Invoice_C" (Math|Transform|MakeTransform (+ (.location _returnvalue) (Math|Vector|MakeVector 0.0 0.0 (* (Variables|Default|GetOffsetAmount) (Variables|Default|GetOffsetCount)))) (Math|Rotator|MakeRotator _roll _pitch (+ _yaw (Math|Random|RandomFloatinRange 0.0 3.6e+02))) "1.000000,1.000000,1.000000") "Undefined" 0 0)
  (Math|Integer|IncrementInt (Variables|Default|GetOffsetCount)
    (:%20%20
      (Utilities|Time|SetTimerbyEvent (delegate Custom|SpawnInvoice) (Math|Random|RandomFloatinRange (Variables|Default|GetMinSpawnTime) (Variables|Default|GetMaxSpawnTime))))))

(event EventBeginPlay
  (bind _invoicespawnlocation (Variables|Default|GetInvoiceSpawnLocation))
  (bind _returnvalue (Transformation|GetWorldTransform _invoicespawnlocation))
  (bind (_roll _pitch _yaw) (Math|Rotator|BreakRotator (.rotation _returnvalue)))
  (Game|SpawnActorfromClass "/Game/Blueprint/BP_Invoice.BP_Invoice_C" (Math|Transform|MakeTransform (+ (.location _returnvalue) (Math|Vector|MakeVector 0.0 0.0 (* (Variables|Default|GetOffsetAmount) (Variables|Default|GetOffsetCount)))) (Math|Rotator|MakeRotator _roll _pitch (+ _yaw (Math|Random|RandomFloatinRange 0.0 3.6e+02))) "1.000000,1.000000,1.000000") "Undefined" 0 0)
  (Math|Integer|IncrementInt (Variables|Default|GetOffsetCount)
    (:%20%20
      (Utilities|Time|SetTimerbyEvent (delegate Custom|SpawnInvoice) (Math|Random|RandomFloatinRange (Variables|Default|GetMinSpawnTime) (Variables|Default|GetMaxSpawnTime))))))

(event Collision|EventActorBeginOverlap
  (params (OtherActor :type Actor%20Object%20Reference)))

(fn ConstructionScript)