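; GlobalScoreManager is an actor that tracks the global score and a countdown level timer.
; AddScore increases the score, while Tick subtracts delta time from the remaining level time.
; Once time drops below zero, it removes the first-person character's game UI and adds a GameOver widget to the viewport.
; The expiry branch has no guard, so it repeats on every later tick.
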(event EventBeginPlay)

(event Collision|EventActorBeginOverlap
  (params (OtherActor :type Actor%20Object%20Reference)))

(event EventTick
  (params (DeltaSeconds :type Float%20%28single-precision%29))
  (bind _output_get (Variables|Default|SetLevelTime (- (Variables|Default|GetLevelTime) DeltaSeconds)))
  (if (< _output_get 0.0)
    (bind _asbp_first_person_character (Utilities|Casting|CastToBP_FirstPersonCharacter (Game|GetPlayerCharacter 0)))
    (Default|RemoveGameUI _asbp_first_person_character)
    (bind _returnvalue (UserInterface|CreateWidget "/Game/UI/GameOver.GameOver_C"))
    (UserInterface|Viewport|AddtoViewport _returnvalue 0)))

(fn ConstructionScript)

(fn AddScore
  (params (ScoreToAdd :type Float%20%28double-precision%29))
  (Variables|Default|SetScore (+ (Variables|Default|GetScore) ScoreToAdd)))