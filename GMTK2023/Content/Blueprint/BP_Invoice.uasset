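; Invoice prop that the player can interact with, showing a randomly chosen action type and a random six-digit number on text renders set at BeginPlay.
; Interact flip-flops the Held flag and toggles the box collision to match, disabling it while held.
; The first interaction also decrements OffsetCount on the BP_InvoiceSpawner found in the level.
; Getters expose the invoice mesh for highlighting and whether its action is completed.
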(event EventBeginPlay
  ;[1 1 1] Set random action type
  (bind _output_get (Variables|Default|SetActionType (Utilities|Enum|ByteToEnumInvoiceAction (Math|Conversions|ToByte(Integer) (Math|Random|RandomIntegerinRange 0 1)))))
  (Rendering|Components|TextRender|SetText (Variables|Default|GetTextRender1) (Utilities|Text|ToText(String) (Utilities|String|EnumtoString _output_get)))
  ;[1 1 1] Generate Random Invoice Number
  (Rendering|Components|TextRender|SetText (Variables|Default|GetTextRender) (Utilities|Text|ToText(String) (Utilities|String|ToString(Integer) (Math|Random|RandomIntegerinRange 100000 999999)))))

(event EventInteract
  (bind _box (Variables|Default|GetBox))
  (Utilities|FlowControl|Sequence
    (:then_0
      (Utilities|FlowControl|FlipFlop
        (:A
          (Collision|SetCollisionEnabled _box "NoCollision")
          (Variables|Default|SetbHeld true))
        (:B
          (Collision|SetCollisionEnabled _box "QueryAndPhysics")
          (Variables|Default|SetbHeld false))))
    (:then_1
      (Utilities|FlowControl|DoOnce false
        (:Completed
          (bind _returnvalue (Actor|GetActorOfClass "/Game/Blueprint/BP_InvoiceSpawner.BP_InvoiceSpawner_C"))
          (Math|Integer|DecrementInt (Variables|/Game/Blueprint/BP_InvoiceSpawner.BP_InvoiceSpawner_C|GetOffsetCount _returnvalue)))))))

(fn ConstructionScript)

(fn GetHighlightMesh
  (return (Variables|Default|GetInvoice)))

(fn HasCompletedAction
  (return (Variables|Default|GetbHasCompletedAction)))