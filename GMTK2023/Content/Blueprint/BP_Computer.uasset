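; BP_Computer is an interactable computer whose health drains periodically on a Tick countdown.
; Interact toggles between locking the first-person character to blend the view onto the computer's widget with a cursor, and restoring normal play.
; Helper functions, not called here, switch damage states using smoke, fire and bluescreen visuals; ComputerAlive also sets health to zero.
; GetHighlightMesh exposes the monitor for highlighting.
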(event EventTick
  (params (DeltaSeconds :type Float%20%28single-precision%29))
  (bind _output_get (Variables|Default|SetHealthDecreaseTimer (- (Variables|Default|GetHealthDecreaseTimer) DeltaSeconds)))
  (if (<= _output_get 0.0)
    (Variables|Default|SetComputerHealth (Math|Integer|Max(Integer) (- (Variables|Default|GetComputerHealth) 5)))
    (Variables|Default|SetHealthDecreaseTimer (Variables|Default|GetHealthDecreaseTime))))

(event EventInteract
  (bind _returnvalue (Game|GetPlayerController 0))
  (bind _returnvalue_2 (Game|GetPlayerController 0))
  (bind _returnvalue_3 (Game|GetPlayerController 0))
  (Utilities|FlowControl|FlipFlop
    (:A
      (bind _asbp_first_person_character (Utilities|Casting|CastToBP_FirstPersonCharacter (Game|GetPlayerCharacter 0)))
      (Variables|/Game/FirstPerson/Blueprints/BP_FirstPersonCharacter.BP_FirstPersonCharacter_C|SetbCanMove _asbp_first_person_character false)
      (Variables|/Game/FirstPerson/Blueprints/BP_FirstPersonCharacter.BP_FirstPersonCharacter_C|SetbCanLook _asbp_first_person_character false)
      (Variables|/Script/Engine.PlayerController|SetbShowMouseCursor _returnvalue_3 true)
      (Game|Player|SetViewTargetwithBlend _returnvalue_2 self 0.5 "VTBlend_Linear" 0.0 false)
      (Input|SetInputModeGameandUI _returnvalue_2 (UserInterface|GetWidget (Variables|Default|GetWidget)) "DoNotLock" true false))
    (:B
      (bind _asbp_first_person_character_2 (Utilities|Casting|CastToBP_FirstPersonCharacter (Game|GetPlayerCharacter 0)))
      (Variables|/Game/FirstPerson/Blueprints/BP_FirstPersonCharacter.BP_FirstPersonCharacter_C|SetbCanMove _asbp_first_person_character_2 true)
      (Variables|/Game/FirstPerson/Blueprints/BP_FirstPersonCharacter.BP_FirstPersonCharacter_C|SetbCanLook _asbp_first_person_character_2 true)
      (Variables|/Script/Engine.PlayerController|SetbShowMouseCursor _returnvalue_3 false)
      (Game|Player|SetViewTargetwithBlend _returnvalue (Game|GetPlayerCharacter 0) 0.5 "VTBlend_Linear" 0.0 false)
      (Input|SetInputModeGameOnly _returnvalue false))))

(fn ConstructionScript)

(fn ComputerDeath
  (Development|SetHiddeninGame (Variables|Default|GetWidget) true false)
  (Development|SetHiddeninGame (Variables|Default|GetBluescreen) false false)
  (bind _returnvalue (Effects|SpawnEmitteratLocation "/Game/StarterContent/Particles/P_Fire.P_Fire" (Transformation|GetWorldLocation (Variables|Default|GetMonitor))))
  (Variables|Default|SetFireParticles _returnvalue))

(fn ComputerAlive
  (Development|SetHiddeninGame (Variables|Default|GetWidget) false false)
  (Development|SetHiddeninGame (Variables|Default|GetBluescreen) true false)
  (Variables|Default|SetComputerHealth 0)
  (Components|DestroyComponent (Variables|Default|GetFireParticles)))

(fn ComputerHalfAlive
  (Variables|Default|GetSmokeParticles
    (:then)
    (:else
      (bind _returnvalue (Effects|SpawnEmitteratLocation "/Game/StarterContent/Particles/P_Smoke.P_Smoke" (Transformation|GetWorldLocation (Variables|Default|GetMonitor)) "0, 0, 0" "0.500000,0.500000,0.500000"))
      (Variables|Default|SetSmokeParticles _returnvalue))))

(fn TryClearSmoke
  (bind _smokeparticles (Variables|Default|GetSmokeParticles)
    (:then
      (Components|DestroyComponent _smokeparticles))
    (:else)))

(fn GetHighlightMesh
  (return (Variables|Default|GetMonitor)))