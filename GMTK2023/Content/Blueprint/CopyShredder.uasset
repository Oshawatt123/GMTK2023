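; Interactable copier or shredder station that consumes the invoice held by the player and scores whether it was brought to the right machine.
; Interact plays the audio, destroys the held BP_Invoice and compares its ActionType with the station's Action.
; A match adds points and a correct count on the GlobalScoreManager found at BeginPlay, while a mismatch deducts points and counts a failure.
; It exposes its mesh for highlighting, but the IsCopier mesh swap is disconnected.
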(event EventInteract
  (bind _scoremanager (Variables|Default|GetScoreManager))
  (bind _asbp_first_person_character (Utilities|Casting|CastToBP_FirstPersonCharacter (Game|GetPlayerCharacter 0)))
  (bind _asbp_invoice (Utilities|Casting|CastToBP_Invoice (Variables|/Game/FirstPerson/Blueprints/BP_FirstPersonCharacter.BP_FirstPersonCharacter_C|GetHeldActor _asbp_first_person_character)))
  (Audio|Components|Audio|Play (Variables|Default|GetAudio) 0.0)
  (bind _output_get (Variables|Default|SetInvoiceAction (Variables|/Game/Blueprint/BP_Invoice.BP_Invoice_C|GetActionType _asbp_invoice)))
  (Actor|DestroyActor _asbp_invoice)
  (Variables|/Game/FirstPerson/Blueprints/BP_FirstPersonCharacter.BP_FirstPersonCharacter_C|SetHeldActor _asbp_first_person_character 0)
  (if (Utilities|Enum|Equal(Enum) (Variables|Default|GetAction) _output_get)
    (Default|AddScore _scoremanager 5.0)
    (Math|Integer|IncrementInt (Variables|/Game/Blueprint/GlobalScoreManager.GlobalScoreManager_C|GetCorrectInvoices _scoremanager))
    (else
      (Default|AddScore _scoremanager -1e+01)
      (Math|Integer|IncrementInt (Variables|/Game/Blueprint/GlobalScoreManager.GlobalScoreManager_C|GetFailedInvoices _scoremanager)))))

(event EventBeginPlay
  (Audio|Components|Audio|Stop (Variables|Default|GetAudio))
  (bind _returnvalue (Actor|GetActorOfClass "/Game/Blueprint/GlobalScoreManager.GlobalScoreManager_C"))
  (Variables|Default|SetScoreManager _returnvalue))

(fn ConstructionScript)

(fn GetHighlightMesh
  (return (Variables|Default|GetStaticMesh)))