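; Coffee machine actor that, on Interact, restores the first-person character's Sanity to full once its cooldown timer has run out.
; Tick counts the timer down, and a successful use restarts it and increments CorrectCoffee on the GlobalScoreManager found at BeginPlay.
; A DoOnce on Tick increments FailedCoffee without checking the timer, so it fires on the first tick and again after each successful use resets it.
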(event EventBeginPlay
  (bind _returnvalue (Actor|GetActorOfClass "/Game/Blueprint/GlobalScoreManager.GlobalScoreManager_C"))
  (Variables|Default|SetGlobalScoreManager _returnvalue))

(event Collision|EventActorBeginOverlap
  (params (OtherActor :type Actor%20Object%20Reference)))

(event EventTick
  (params (DeltaSeconds :type Float%20%28single-precision%29))
  (Variables|Default|SetCoffeeMachineTimer (- (Variables|Default|GetCoffeeMachineTimer) DeltaSeconds))
  (Utilities|FlowControl|DoOnce false
    (:Completed
      (Math|Integer|IncrementInt (Variables|/Game/Blueprint/GlobalScoreManager.GlobalScoreManager_C|GetFailedCoffee (Variables|Default|GetGlobalScoreManager))))))

(event EventInteract
  (if (<= (Variables|Default|GetCoffeeMachineTimer) 0.0)
    (bind _asbp_first_person_character (Utilities|Casting|CastToBP_FirstPersonCharacter (Game|GetPlayerCharacter 0)))
    (Variables|/Game/FirstPerson/Blueprints/BP_FirstPersonCharacter.BP_FirstPersonCharacter_C|SetSanity _asbp_first_person_character 1e+02)
    (Variables|Default|SetCoffeeMachineTimer (Variables|Default|GetCoffeeMachineTime))
    (Math|Integer|IncrementInt (Variables|/Game/Blueprint/GlobalScoreManager.GlobalScoreManager_C|GetCorrectCoffee (Variables|Default|GetGlobalScoreManager))
      (:%20%20
        (Utilities|FlowControl|DoOnce false) ; enters at Reset
      ))))

(fn ConstructionScript)