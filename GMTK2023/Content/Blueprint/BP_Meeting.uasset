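; BP_Meeting is an interactable actor for a timed meeting that the player must keep up with by taking notes.
; Tick compares GlobalScoreManager's LevelTime to a start and end window, showing MeetingUI once and removing it afterwards.
; During the meeting, an expired note timer repeatedly applies score loss and counts failures.
; Interact refreshes that timer, awards score, counts a success and starts an interaction cooldown.
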(event EventBeginPlay
  (bind _returnvalue (Actor|GetActorOfClass "/Game/Blueprint/GlobalScoreManager.GlobalScoreManager_C"))
  (Variables|Default|SetGlobalScoreManager _returnvalue))

(event EventTick
  (params (DeltaSeconds :type Float%20%28single-precision%29))
  (bind _globalscoremanager (Variables|Default|GetGlobalScoreManager))
  (Variables|Default|SetNoteTimer (Math|Float|Max(Float) (- (Variables|Default|GetNoteTimer) DeltaSeconds) 0.0))
  (if (>= (Variables|/Game/Blueprint/GlobalScoreManager.GlobalScoreManager_C|GetLevelTime (Variables|Default|GetGlobalScoreManager)) (Variables|Default|GetStartTime))
    (Utilities|FlowControl|Sequence
      (:then_0
        (if (>= (Variables|/Game/Blueprint/GlobalScoreManager.GlobalScoreManager_C|GetLevelTime (Variables|Default|GetGlobalScoreManager)) (Variables|Default|GetEndTime))
          ;[1 1 1] Meeting ended
          (Variables|Default|SetbMeetingActive false)
          (Utilities|FlowControl|DoOnce false
            (:Completed
              (Widget|RemovefromParent (stale _returnvalue))))
          (else
            ;[1 1 1] Meeting Active
            (Variables|Default|SetbMeetingActive true)
            (if (<= (Variables|Default|GetNoteTimer) 0.0)
              (Utilities|FlowControl|Sequence
                (:then_0
                  (Utilities|FlowControl|DoOnce false :!label _label
                    (:Completed
                      (Default|AddScore _globalscoremanager (Variables|Default|GetScoreLossPerSecond) :!label _label_2)
                      (Math|Integer|IncrementInt (Variables|/Game/Blueprint/GlobalScoreManager.GlobalScoreManager_C|GetFailedMeetings _globalscoremanager)))))
                (:then_1
                  (bind _output_get (Variables|Default|SetScoreLossTimer (- (Variables|Default|GetScoreLossTimer) DeltaSeconds)))
                  (if (<= _output_get 0.0)
                    (Variables|Default|SetScoreLossTimer 1.0)
                    (goto _label_2))))
              (else
                (Utilities|FlowControl|Sequence
                  (:then_0
                    (goto _label Reset))
                  (:then_1
                    (bind _output_get_2 (Variables|Default|SetNoteInteractTimer (- (Variables|Default|GetNoteInteractTimer) DeltaSeconds)))
                    (if (<= _output_get_2 0.0)
                      (Variables|Default|SetbCanInteractWithNote true)))))))))
      (:then_1
        (Utilities|FlowControl|DoOnce false
          (:Completed
            (bind _returnvalue (UserInterface|CreateWidget "/Game/UI/MeetingUI.MeetingUI_C"))
            (UserInterface|Viewport|AddtoViewport _returnvalue 0)
            (Variables|Default|SetNoteTimer (Variables|Default|GetNoteTime))))))))

(event EventInteract
  (bind _globalscoremanager (Variables|Default|GetGlobalScoreManager))
  (if (Variables|Default|GetbCanInteractWithNote)
    (if (Variables|Default|GetbMeetingActive)
      (Variables|Default|SetNoteTimer (Variables|Default|GetNoteTime))
      (Default|AddScore _globalscoremanager 4e+01)
      (Math|Integer|IncrementInt (Variables|/Game/Blueprint/GlobalScoreManager.GlobalScoreManager_C|GetCorrectMeetings _globalscoremanager)
        (:%20%20
          (Variables|Default|SetbCanInteractWithNote false)
          (Variables|Default|SetNoteInteractTimer (Variables|Default|GetNoteInteractTime)))))))

(fn ConstructionScript)

(fn GetHighlightMesh
  (return (Variables|Default|GetStaticMesh)))